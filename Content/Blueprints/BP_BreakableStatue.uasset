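; Breakable statue that swaps its static mesh for a Chaos Geometry Collection when damage or hit impulse exceeds a threshold.
; SwapToDestructible carries linear and angular velocity over to the collection.
; Damage breaks apply external strain and fire a short-lived FS_MasterField at a computed hit transform, while collision breaks apply strain and the hit impulse at the impact point.
; Broken pieces switch to the Debris collision profile through the Chaos break event.
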(event OnChaosBreakEvent(GeometryCollection)
  (params (BreakEvent :type Chaos%20Break%20Event%20Structure%20%28by%20ref%29))
  (Class|GeometryCollectionComponent|SetPerParticleCollisionProfileName (Variables|Default|GetGeometryCollection) (Utilities|Array|MakeArray (.Index (Utilities|Struct|BreakChaosBreakEvent BreakEvent))) "Debris"))

(event Custom|CustomEvent
  (params (HitComponent :type Primitive%20Component%20Object%20Reference) (OtherActor :type Actor%20Object%20Reference) (OtherComp :type Primitive%20Component%20Object%20Reference) (NormalImpulse :type Vector) (Hit :type Hit%20Result%20Structure%20%28by%20ref%29))
  (bind _impactpoint (Collision|BreakHitResult Hit))
  (if (> (Math|Vector|VectorLength NormalImpulse) (Variables|Default|GetMinImpulseToBreak))
    (CallFunction|SwaptoDestructible)
    (Class|GeometryCollectionComponent|ApplyExternalStrain (Variables|Default|GetGeometryCollection) 0 _impactpoint 5.0 0 1.0 (Variables|Default|GetOnHitStrain))
    (Physics|AddImpulseatLocation (Variables|Default|GetGeometryCollection) NormalImpulse _impactpoint "None")))

(event Custom|OnTakePointDamage_Event
  (params (DamagedActor :type Actor%20Object%20Reference) (Damage :type Float%20%28single-precision%29) (InstigatedBy :type Controller%20Object%20Reference) (HitLocation :type Vector) (FHitComponent :type Primitive%20Component%20Object%20Reference) (BoneName :type Name) (ShotFromDirection :type Vector) (DamageType :type Damage%20Type%20Object%20Reference) (DamageCauser :type Actor%20Object%20Reference))
  (if (not (Variables|Default|GetDestroyed))
    (Variables|Default|SetHitZoneTransform (Math|Transform|MakeTransform (.ImpactPoint (Collision|BreakHitResult (stale Custom|OnTakeRadialDamage_Event HitInfo))) (Math|Conversions|RotationFromXVector (Math|Vector|NegateVector (.ImpactNormal (Collision|BreakHitResult (stale Custom|OnTakeRadialDamage_Event HitInfo)))))))
    (if (> (stale Custom|OnTakeRadialDamage_Event Damage) (Variables|Default|GetMinDamageToBreak))
      (CallFunction|SwaptoDestructible)
      (Class|GeometryCollectionComponent|ApplyExternalStrain (Variables|Default|GetGeometryCollection) 0 (Transformation|GetActorLocation) 5.0 0 1.0 (Variables|Default|GetOnHitStrain))
      (bind _returnvalue (Game|SpawnActorfromClass "/Engine/EditorResources/FieldNodes/FS_MasterField.FS_MasterField_C" (Variables|Default|GetHitZoneTransform) "AlwaysSpawn" "MultiplyWithRoot" 0 0))
      (Default|CETrigger _returnvalue)
      (Actor|DestroyActor _returnvalue)
      (Class|PrimitiveComponent|SetWalkableSlopeOverride (Variables|Default|GetGeometryCollection) (Utilities|Struct|MakeWalkableSlopeOverride "WalkableSlope_Unwalkable" 0.0)))))

(event Custom|OnTakeRadialDamage_Event
  (params (DamagedActor :type Actor%20Object%20Reference) (Damage :type Float%20%28single-precision%29) (DamageType :type Damage%20Type%20Object%20Reference) (Origin :type Vector) (HitInfo :type Hit%20Result%20Structure%20%28by%20ref%29) (InstigatedBy :type Controller%20Object%20Reference) (DamageCauser :type Actor%20Object%20Reference))
  (bind (_bblockinghit _binitialoverlap _time _distance _location _impactpoint _normal _impactnormal) (Collision|BreakHitResult HitInfo))
  (if (not (Variables|Default|GetDestroyed))
    (Variables|Default|SetHitZoneTransform (Math|Transform|MakeTransform _impactpoint (Math|Conversions|RotationFromXVector (Math|Vector|NegateVector _impactnormal))))
    (if (> Damage (Variables|Default|GetMinDamageToBreak))
      (CallFunction|SwaptoDestructible)
      (Class|GeometryCollectionComponent|ApplyExternalStrain (Variables|Default|GetGeometryCollection) 0 (Transformation|GetActorLocation) 5.0 0 1.0 (Variables|Default|GetOnHitStrain))
      (bind _returnvalue (Game|SpawnActorfromClass "/Engine/EditorResources/FieldNodes/FS_MasterField.FS_MasterField_C" (Variables|Default|GetHitZoneTransform) "AlwaysSpawn" "MultiplyWithRoot" 0 0))
      (Default|CETrigger _returnvalue)
      (Actor|DestroyActor _returnvalue)
      (Class|PrimitiveComponent|SetWalkableSlopeOverride (Variables|Default|GetGeometryCollection) (Utilities|Struct|MakeWalkableSlopeOverride "WalkableSlope_Unwalkable" 0.0)))))

(event Custom|OnTakeNormalDamage
  (params (DamagedActor :type Actor%20Object%20Reference) (Damage :type Float%20%28single-precision%29) (DamageType :type Damage%20Type%20Object%20Reference) (InstigatedBy :type Controller%20Object%20Reference) (DamageCauser :type Actor%20Object%20Reference))
  (if (not (Variables|Default|GetDestroyed))
    (Variables|Default|SetHitZoneTransform (Math|Transform|MakeTransform (Transformation|GetWorldLocation (Variables|Default|GetExplosionPoint))))
    (if (> (stale Custom|OnTakeRadialDamage_Event Damage) (Variables|Default|GetMinDamageToBreak))
      (CallFunction|SwaptoDestructible)
      (Class|GeometryCollectionComponent|ApplyExternalStrain (Variables|Default|GetGeometryCollection) 0 (Transformation|GetActorLocation) 5.0 0 1.0 (Variables|Default|GetOnHitStrain))
      (bind _returnvalue (Game|SpawnActorfromClass "/Engine/EditorResources/FieldNodes/FS_MasterField.FS_MasterField_C" (Variables|Default|GetHitZoneTransform) "AlwaysSpawn" "MultiplyWithRoot" 0 0))
      (Default|CETrigger _returnvalue)
      (Actor|DestroyActor _returnvalue)
      (Class|PrimitiveComponent|SetWalkableSlopeOverride (Variables|Default|GetGeometryCollection) (Utilities|Struct|MakeWalkableSlopeOverride "WalkableSlope_Unwalkable" 0.0)))))

(event EventBeginPlay
  (Collision|BindEventtoOnComponentHit (Variables|Default|GetStaticMesh) (delegate Custom|CustomEvent))
  (EventDispatchers|AssignOnTakePointDamage (delegate Custom|OnTakePointDamage_Event))
  (EventDispatchers|AssignOnTakeRadialDamage (delegate Custom|OnTakeRadialDamage_Event))
  (EventDispatchers|BindEventtoOnTakeAnyDamage (delegate Custom|OnTakeNormalDamage)))

(fn ConstructionScript)

(fn SwaptoDestructible
  (bind _staticmesh (Variables|Default|GetStaticMesh))
  (bind _geometrycollection (Variables|Default|GetGeometryCollection))
  (bind _staticmesh_2 (Variables|Default|GetStaticMesh))
  (bind _geometrycollection_2 (Variables|Default|GetGeometryCollection))
  (Utilities|FlowControl|Sequence
    (:then_0
      (Variables|Default|SetDestroyed true))
    (:then_1
      ;[0.15 0.04222 0.03236 0.5] Storing old velocity
      (bind _returnvalue (Physics|GetPhysicsLinearVelocity _staticmesh "None"))
      (LocalVariables|SetLinearVelocity _returnvalue)
      (LocalVariables|SetAngularVelocity (Class|PrimitiveComponent|GetPhysicsAngularVelocityinRadians _staticmesh "None")))
    (:then_2
      ;[0.09004 0.15 0.04801 0.5] Disabling old mesh.
      (Physics|SetSimulatePhysics _staticmesh_2 false)
      (Collision|SetCollisionEnabled _staticmesh_2 "NoCollision")
      (Rendering|SetVisibility _staticmesh_2 false false))
    (:then_3
      ;[0.15 0.1272 0.02932 0.5] Enabling Collection
      (Collision|SetCollisionEnabled _geometrycollection "QueryAndPhysics")
      (Rendering|SetVisibility _geometrycollection true false)
      (Physics|SetSimulatePhysics _geometrycollection true))
    (:then_4
      ;[0.05967 0.1211 0.15 0.5] Setting new velocities
      (Physics|SetPhysicsLinearVelocity _geometrycollection_2 (LocalVariables|GetLinearVelocity) false "None")
      (Class|PrimitiveComponent|SetPhysicsAngularVelocityinRadians _geometrycollection_2 (LocalVariables|GetAngularVelocity) false "None"))))